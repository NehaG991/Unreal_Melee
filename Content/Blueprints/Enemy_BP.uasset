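; Enemy that the player can assassinate when inside its AssassinateCollision volume.
; Overlap by a component tagged "playerCap" sets CanAssassinate and shows a custom-depth stencil outline, which separate events can also toggle.
; Assassinate triggers the gated death montage and always returns the AssassinationPoint location and rotation to the caller.
; A montage notify calls Death, which enables ragdoll physics, clears the outline and sets a short lifespan.
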(event OnComponentBeginOverlap(AssassinateCollision)
  (params (OverlappedComponent :type Primitive%20Component%20Object%20Reference) (OtherActor :type Actor%20Object%20Reference) (OtherComp :type Primitive%20Component%20Object%20Reference) (OtherBodyIndex :type Integer) (bFromSweep :type Boolean) (SweepResult :type Hit%20Result%20Structure%20%28by%20ref%29))
  (if (Components|ComponentHasTag OtherComp "playerCap")
    (Variables|Default|SetCanAssassinate true)
    (Rendering|SetRenderCustomDepth (Variables|Character|GetMesh) true)))

(event OnComponentEndOverlap(AssassinateCollision)
  (params (OverlappedComponent :type Primitive%20Component%20Object%20Reference) (OtherActor :type Actor%20Object%20Reference) (OtherComp :type Primitive%20Component%20Object%20Reference) (OtherBodyIndex :type Integer))
  (if (Components|ComponentHasTag OtherComp "playerCap")
    (Variables|Default|SetCanAssassinate false)
    (Rendering|SetRenderCustomDepth (Variables|Character|GetMesh) false)))

(event Custom|Assassination
  (if (Variables|Default|GetCanAssassinate)
    (Development|PrintString "Assassinated")
    (Animation|Montage|PlayMontage (Variables|Character|GetMesh) "/Game/Characters/Enemy/AssassinateDeath_Montage.AssassinateDeath_Montage"
      (:OnNotifyBegin
        (CallFunction|Death)))))

(event Custom|On%20Outline
  ;[0 0 0] Outline
  (Rendering|SetRenderCustomDepth (Variables|Character|GetMesh) true))

(event Custom|Off%20Outline
  ;[0 0 0] Outline
  (Rendering|SetRenderCustomDepth (Variables|Character|GetMesh) false))

(event EventBeginPlay
  (Rendering|SetCustomDepthStencilValue (Variables|Character|GetMesh) 2))

(event Collision|EventActorBeginOverlap
  (params (OtherActor :type Actor%20Object%20Reference)))

(event EventTick
  (params (DeltaSeconds :type Float%20%28single-precision%29)))

(event EventTurnonOutline
  ;[0 0 0] Outline
  (CallFunction|OnOutline))

(event EventTurnOffOutline
  ;[0 0 0] Outline
  (CallFunction|OffOutline))

(fn ConstructionScript)

(fn Death
  (Collision|SetCollisionEnabled (Variables|Character|GetMesh) "PhysicsOnly")
  (Physics|SetSimulatePhysics (Variables|Character|GetMesh) true)
  (Actor|SetLifeSpan 5.0)
  (CallFunction|TurnOffOutline))

(fn Assassinate
  (bind _assassinationpoint (Variables|Default|GetAssassinationPoint))
  (CallFunction|Assassination)
  (return (Transformation|GetWorldLocation _assassinationpoint) (Transformation|GetWorldRotation _assassinationpoint)))