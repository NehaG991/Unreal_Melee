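; Weapon item Blueprint, a child item actor that can be highlighted and interacted with once in the world.
; BeginPlay runs the parent logic, sets the item type and assigns its mesh to the InteractableObject component.
; Outline events toggle Custom Depth rendering on that mesh, turning it on only while the item is interactable.
; Interacting currently just prints a debug string, clears the outline and disables further interaction, with no pickup or equip logic.
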(event Custom|Interacting
  ;[0 0 0] Interacting Logic
  (if (Variables|Default|GetInteractable)
    (Development|PrintString "Interacting")
    (Rendering|SetRenderCustomDepth (Variables|Default|GetInteractableObject) false)
    (Variables|Default|SetInteractable false)))

(event Custom|On%20Outline
  ;[0 0 0] Outline Logic
  (if (Variables|Default|GetInteractable)
    (Rendering|SetRenderCustomDepth (Variables|Default|GetInteractableObject) true)))

(event Custom|Off%20Outline
  ;[0 0 0] Outline Logic
  (Rendering|SetRenderCustomDepth (Variables|Default|GetInteractableObject) false))

(event EventBeginPlay
  (|CallParentFunction)
  (Variables|Default|SetType "NewEnumerator0")
  (Components|StaticMesh|SetStaticMesh (Variables|Default|GetInteractableObject) (Variables|Default|GetMesh)))

(event Collision|EventActorBeginOverlap
  (params (OtherActor :type Actor%20Object%20Reference))
  (|CallParentFunction OtherActor) ; This node is disabled and will not be called.\nDrag off pins to build functionality.
)

(event EventTick
  (params (DeltaSeconds :type Float%20%28single-precision%29))
  (|CallParentFunction DeltaSeconds) ; This node is disabled and will not be called.\nDrag off pins to build functionality.
)

(event EventInteract
  ;[0 0 0] Interacting Logic
  (CallFunction|Interacting))

(event EventTurnonOutline
  ;[0 0 0] Outline Logic
  (CallFunction|OnOutline))

(event EventTurnOffOutline
  ;[0 0 0] Outline Logic
  (CallFunction|OffOutline))

(fn ConstructionScript
  (|CallParentFunction))